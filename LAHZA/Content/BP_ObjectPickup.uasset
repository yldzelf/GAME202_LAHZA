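; BP_ObjectPickup is an object the third-person character picks up and drops with the Interact input.
; A detection capsule stores the overlapping character as PlayerRef and clears it when that character leaves.
; While PlayerRef is valid, each press alternates through a FlipFlop between snapping to the ObjectSocket on the character's mesh and detaching in place, keeping world transform.
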(event `InputAction|Interact`
  (params (Key :type "Key Structure"))
  (:`Pressed`
    (`/Engine/EditorBlueprintResources/StandardMacros.IsValid` (`self.PlayerRef`)
      (:`Is Valid`
        (`/Engine/EditorBlueprintResources/StandardMacros.FlipFlop`
          (:`A`
            (`self.K2_AttachToComponent` (`Character.Mesh` (`self.PlayerRef`)) "ObjectSocket" "SnapToTarget" "SnapToTarget" "KeepRelative"))
          (:`B`
            (`self.K2_DetachFromActor` "KeepWorld" "KeepWorld" "KeepWorld")))))))

(event `self.PlayerDetecCapsule.OnComponentBeginOverlap`
  (params (OverlappedComponent :type "PrimitiveComponent Object Reference") (OtherActor :type "Actor Object Reference") (OtherComp :type "PrimitiveComponent Object Reference") (OtherBodyIndex :type Integer) (bFromSweep :type Boolean) (SweepResult :type "HitResult Structure (by ref)"))
  (bind _asbp_third_person_character (cast `/Game/ThirdPerson/Blueprints/BP_ThirdPersonCharacter` OtherActor))
  (set `self.PlayerRef` _asbp_third_person_character))

(event `self.PlayerDetecCapsule.OnComponentEndOverlap`
  (params (OverlappedComponent :type "PrimitiveComponent Object Reference") (OtherActor :type "Actor Object Reference") (OtherComp :type "PrimitiveComponent Object Reference") (OtherBodyIndex :type Integer))
  (cast `/Game/ThirdPerson/Blueprints/BP_ThirdPersonCharacter` OtherActor)
  (set `self.PlayerRef` null))

(fn `UserConstructionScript`)